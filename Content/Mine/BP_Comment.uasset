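; BP_Comment is an actor that shows a written note in the level through two text render components.
; Its construction script sets one text render from the Header variable and the other from the Container variable.
; Unconnected leftover nodes sketch a sphere trace at the actor's location and a rotation toward the hit normal, but they never run.
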(event EventBeginPlay)

(event EventTick
  (params (DeltaSeconds :type Float%20%28single-precision%29)))

(fn ConstructionScript
  (Utilities|FlowControl|Sequence
    (:then_1
      (Rendering|Components|TextRender|SetText (Variables|Default|GetTextRender1) (Utilities|Text|ToText(String) (Variables|Default|GetContainer)))
      (Rendering|Components|TextRender|SetText (Variables|Default|GetTextRender) (Utilities|Text|ToText(String) (Variables|Default|GetHeader))))))